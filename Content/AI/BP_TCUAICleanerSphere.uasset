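; AI-controlled cleaner sphere that wanders around the level at random.
; From BeginPlay, RandomMove picks a reachable point within a radius of its current location and uses AI MoveTo, repeating only on success, so a failed move ends the wandering.
; A Hit event briefly turns on physics simulation on the capsule, then switches it off after a delay.
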(event Custom|Random%20Move
  (AI|AIMoveTo self (.RandomLocation (AI|Navigation|GetRandomReachablePointinRadius (Transformation|GetActorLocation) 1e+03 0 0)) 0 5.0 false
    (:OnSuccess
      (CallFunction|RandomMove))))

(event EventBeginPlay
  (CallFunction|RandomMove))

(event Collision|EventHit
  (params (MyComp :type Primitive%20Component%20Object%20Reference) (Other :type Actor%20Object%20Reference) (OtherComp :type Primitive%20Component%20Object%20Reference) (bSelfMoved :type Boolean) (HitLocation :type Vector :default "0, 0, 0") (HitNormal :type Vector :default "0, 0, 0") (NormalImpulse :type Vector :default "0, 0, 0") (Hit :type Hit%20Result%20Structure%20%28by%20ref%29))
  (Physics|SetSimulatePhysics (Variables|Collision|GetCapsuleComponent) true)
  (Utilities|FlowControl|Delay 1.5)
  (Physics|SetSimulatePhysics (Variables|Collision|GetCapsuleComponent) false))

(fn ConstructionScript)