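; BP_TCUCharacter is a character Blueprint whose only active logic toggles the game's pause menu from the Pause Game input action.
; It creates a WBP_PausedMenu widget behind a validity check and stores it as PauseMenuREF.
; Each press flips the paused state, adding or removing the menu, showing or hiding the mouse cursor, and switching between Game-and-UI and Game-Only input modes.
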(event EventBeginPlay)

(event Input|ActionEvents|InputActionPauseGame
  (params (Key :type Key%20Structure :default "None"))
  (bind _returnvalue (Game|GetPlayerController 0))
  ;[1 1 1] Pause/un-pause game
  (:Pressed
    (Utilities|IsValid 0
      (:Is%20Valid
        _)
      (:Is%20Not%20Valid
        (bind _returnvalue_2 (UserInterface|CreateWidget "/Game/UI/WBP_PausedMenu.WBP_PausedMenu_C"))
        (Variables|Default|SetPause%20Menu%20REF _returnvalue_2)))
    (if (Game|IsGamePaused)
      (Widget|RemovefromParent (Variables|Default|GetPause%20Menu%20REF))
      (Game|SetGamePaused false)
      (Variables|/Script/Engine.PlayerController|SetbShowMouseCursor _returnvalue false)
      (Input|SetInputModeGameOnly _returnvalue false)
      (else
        (UserInterface|Viewport|AddtoViewport (Variables|Default|GetPause%20Menu%20REF) 0)
        (Game|SetGamePaused true)
        (Variables|/Script/Engine.PlayerController|SetbShowMouseCursor _returnvalue true)
        (Input|SetInputModeGameandUI _returnvalue (Variables|Default|GetPause%20Menu%20REF) "LockInFullscreen" false false)))))

(fn ConstructionScript)